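; BP_NewCharacter is a player character Blueprint whose graphs hold no active logic.
; An unconnected debug fragment checks the CharAttribute equipped weapon, then line-traces on Visibility from the weapon's location along the control rotation.
; That fragment draws the trace and prints the hit actor's name, but no event triggers it.
; The overlap event and construction script are empty.
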(event `EnhancedInput|/Game/Input/IA_Shot`
  (params (ActionValue :type Boolean) (ElapsedSeconds :type "Float (double-precision)") (TriggeredSeconds :type "Float (double-precision)") (InputAction :type "InputAction Object Reference" :default "/Game/Input/IA_Shot.IA_Shot")))

(fn `UserConstructionScript`)