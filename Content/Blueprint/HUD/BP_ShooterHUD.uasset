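; Shooter HUD Blueprint that draws a dynamic four-piece crosshair at the screen center.
; Each DrawHUD offsets top, bottom, left and right textures from the center by the PlayerCharacter's spread multiplier times a maximum spread.
; BeginPlay caches the character only if the reference is already valid.
; When it is invalid, DrawHUD casts the player pawn but sets the reference to None, so the cast repeats on later draws.
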(event `self.ReceiveBeginPlay`
  ;[1 1 1] 플레이어 캐릭터 레퍼런스 얻기
  (`self.ShooterCharacter`
    (:`then`
      (bind _asplayer_character (cast `PlayerCharacter` (`GameplayStatics.GetPlayerPawn` 0)))
      (set `self.ShooterCharacter` _asplayer_character))
    (:`else`)))

(event `self.ReceiveDrawHUD`
  (params (SizeX :type Integer) (SizeY :type Integer))
  (bind (_x _y) (`KismetMathLibrary.BreakVector2D` (`self.CrosshairBaseCenter`)))
  (bind (_x_2 _y_2) (`KismetMathLibrary.BreakVector2D` (`self.CrosshairBaseCenter`)))
  (bind (_x_3 _y_3) (`KismetMathLibrary.BreakVector2D` (`self.CrosshairBaseCenter`)))
  (bind (_x_4 _y_4) (`KismetMathLibrary.BreakVector2D` (`self.CrosshairBaseCenter`)))
  (bind (_x_5 _y_5) (`KismetMathLibrary.BreakVector2D` (`self.CrossHairLocation`)))
  (bind (_x_6 _y_6) (`KismetMathLibrary.BreakVector2D` (`self.Screen Center`)))
  ;[1 1 1] 스크린 중앙 구하기
  (set `self.Screen Center` (`KismetMathLibrary.MakeVector2D` (`KismetMathLibrary.Conv_IntToDouble` (/ SizeX 2)) (`KismetMathLibrary.Conv_IntToDouble` (/ SizeY 2))))
  (set `self.CrossHairLocation` (`KismetMathLibrary.MakeVector2D` _x_6 _y_6))
  ;[1 1 1] 플레이어 컨트롤러가 유효한지 확인
  (`self.ShooterCharacter`
    (:`then`
      _)
    (:`else`
      (bind _asplayer_character (cast `PlayerCharacter` (`GameplayStatics.GetPlayerPawn` 0)))
      (set `self.ShooterCharacter` null)))
  ;[1 1 1] 크로스헤어 스프래드 멀티플라이어 GET
  (set `self.CrosshairSpreadMultiplier` (`PlayerCharacter.GetCrosshairSpreadMultiplier` _asplayer_character))
  ;[1 1 1] 크로스헤어 중심 설정
  (set `self.CrosshairBaseCenter` (`KismetMathLibrary.MakeVector2D` (- _x_5 (`self.CrossHairHalfWidth`)) (- _y_5 (`self.CrossHairHalfHeight`))))
  (`self.DrawTexture` "/Game/Assets/HUD/Crosshair_Quad_9_Bottom.Crosshair_Quad_9_Bottom" _x_3 (+ _y_3 (* (`self.CrosshairSpreadMultiplier`) (`self.CrosshairSpreadMax`))) 64.0 64.0 0.0 0.0 1.0 1.0)
  (`self.DrawTexture` "/Game/Assets/HUD/Crosshair_Quad_9_Top.Crosshair_Quad_9_Top" _x_4 (- _y_4 (* (`self.CrosshairSpreadMultiplier`) (`self.CrosshairSpreadMax`))) 64.0 64.0 0.0 0.0 1.0 1.0)
  (`self.DrawTexture` "/Game/Assets/HUD/Crosshair_Quad_9_Right.Crosshair_Quad_9_Right" (+ _x (* (`self.CrosshairSpreadMultiplier`) (`self.CrosshairSpreadMax`))) _y 64.0 64.0 0.0 0.0 1.0 1.0)
  (`self.DrawTexture` "/Game/Assets/HUD/Crosshair_Quad_9_Left.Crosshair_Quad_9_Left" (- _x_2 (* (`self.CrosshairSpreadMultiplier`) (`self.CrosshairSpreadMax`))) _y_2 64.0 64.0 0.0 0.0 1.0 1.0))

(fn `UserConstructionScript`)